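; BP_TankPlayerController is the player controller that handles the tank player's UI and pause menu.
; An AddWidget event creates the player UI widget and adds it to the viewport.
; Escape or R, when the pawn is a BP_TankPawn, creates and caches the pause menu on first use, shows it and the cursor, switches to UI-only input, and pauses the game.
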(event EventBeginPlay)

(event EventTick
  (params (DeltaSeconds :type Float%20%28single-precision%29)))

(event EventAddWidget
  (bind _returnvalue (UserInterface|CreateWidget "/Game/Blueprint/Widgets/WBP_PlayerUI.WBP_PlayerUI_C"))
  (UserInterface|Viewport|AddtoViewport _returnvalue 0))

(event Input|KeyboardEvents|Escape
  (params (Key :type Key%20Structure :default "None"))
  (:Pressed
    (Utilities|Casting|CastToBP_TankPawn (Game|Player|GetPlayerPawn 0))
    (Utilities|IsValid (Variables|Default|GetPauseMenu)
      (:Is%20Valid
        _)
      (:Is%20Not%20Valid
        (bind _returnvalue (UserInterface|CreateWidget "/Game/Blueprint/Widgets/WBP_PauseMenu.WBP_PauseMenu_C" self))
        (Variables|Default|SetPauseMenu _returnvalue)))
    (Variables|Default|SetbShowMouseCursor true)
    (Input|SetInputModeUIOnly self (Variables|Default|GetPauseMenu) "DoNotLock")
    (UserInterface|Viewport|AddtoViewport (Variables|Default|GetPauseMenu) 0)
    (Game|SetGamePaused true)))

(event Input|KeyboardEvents|R
  (params (Key :type Key%20Structure :default "None"))
  (:Pressed
    (Utilities|Casting|CastToBP_TankPawn (Game|Player|GetPlayerPawn 0))
    (Utilities|IsValid (Variables|Default|GetPauseMenu)
      (:Is%20Valid
        _)
      (:Is%20Not%20Valid
        (bind _returnvalue (UserInterface|CreateWidget "/Game/Blueprint/Widgets/WBP_PauseMenu.WBP_PauseMenu_C" self))
        (Variables|Default|SetPauseMenu _returnvalue)))
    (Variables|Default|SetbShowMouseCursor true)
    (Input|SetInputModeUIOnly self (Variables|Default|GetPauseMenu) "DoNotLock")
    (UserInterface|Viewport|AddtoViewport (Variables|Default|GetPauseMenu) 0)
    (Game|SetGamePaused true)))

(fn ConstructionScript)