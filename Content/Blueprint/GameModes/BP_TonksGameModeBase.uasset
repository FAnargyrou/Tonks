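; Game mode for the Tonks tank game that handles the end of a match.
; GameOver shows a WBP_GameOver widget with the LastTankAlive player's name as winner, or an empty name if no valid tank remains.
; It then starts a timer that calls ReturnToMainMenu by name to open the MainMenu level after a short delay.
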(event EventBeginPlay)

(event EventTick
  (params (DeltaSeconds :type Float%20%28single-precision%29)))

(event EventGameOver
  (bind _returnvalue (UserInterface|CreateWidget "/Game/Blueprint/Widgets/WBP_GameOver.WBP_GameOver_C"))
  (if (Utilities|IsValid (Variables|Default|GetLastTankAlive))
    (Default|SetPlayerWon _returnvalue (Variables|/Script/Tonks.BasePawn|GetPlayerName (Variables|Default|GetLastTankAlive)))
    (else
      (Default|SetPlayerWon _returnvalue)))
  (UserInterface|Viewport|AddtoViewport _returnvalue 0)
  (Utilities|Time|SetTimerbyFunctionName 0 "ReturnToMainMenu" 1e+01))

(fn ConstructionScript)

(fn ReturntoMainMenu
  (Game|OpenLevel(byName) "MainMenu"))