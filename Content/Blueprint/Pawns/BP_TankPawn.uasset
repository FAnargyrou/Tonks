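; BP_TankPawn is a tank pawn with a floating health bar widget and a health component.
; On BeginPlay it passes itself to the WBP_TonkHealth widget as its Tonk reference.
; When it takes any damage, it plays the widget's DamageDisplay animation and calls the Health component's CalculateDamage from the animation's Finished pin.
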(event Game|Damage|EventAnyDamage
  (params (Damage :type Float%20%28single-precision%29) (DamageType :type Damage%20Type%20Object%20Reference) (InstigatedBy :type Controller%20Object%20Reference) (DamageCauser :type Actor%20Object%20Reference))
  (bind _aswbp_tonk_health (Utilities|Casting|CastToWBP_TonkHealth (UserInterface|GetUserWidgetObject (Variables|Default|GetFloatingHealthBar))))
  (Components|Animation|PlayAnimation _aswbp_tonk_health (Variables|/Game/Blueprint/Widgets/WBP_TonkHealth.WBP_TonkHealth_C|GetDamageDisplay _aswbp_tonk_health) 0.0
    (:Finished
      (Class|HealthComponent|CalculateDamage (Variables|Default|GetHealth)))))

(event Collision|EventActorBeginOverlap
  (params (OtherActor :type Actor%20Object%20Reference)))

(event EventTick
  (params (DeltaSeconds :type Float%20%28single-precision%29)))

(event EventBeginPlay
  (bind _aswbp_tonk_health (Utilities|Casting|CastToWBP_TonkHealth (UserInterface|GetUserWidgetObject (Variables|Default|GetFloatingHealthBar))))
  (Variables|/Game/Blueprint/Widgets/WBP_TonkHealth.WBP_TonkHealth_C|SetTonk _aswbp_tonk_health self))

(fn ConstructionScript)